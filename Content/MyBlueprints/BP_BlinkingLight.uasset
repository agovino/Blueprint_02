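; BP_BlinkingLight is a light Blueprint that makes its point light flicker by continually varying its intensity at random.
; Each Tick moves the intensity toward a target at a constant PulseRate using FInterpToConstant.
; When the intensity exactly equals the target, a new random target is picked between MinIntensity and MaxIntensity.
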(event EventTick
  (params (DeltaSeconds :type Float%20%28single-precision%29))
  (if (== (Variables|/Script/Engine.LightComponentBase|GetIntensity (Variables|Default|GetPointLightComponent)) (Variables|Default|GetTargetIntensity))
    (Variables|Default|SetTargetIntensity (Math|Random|RandomFloatinRange (Variables|Default|GetMinIntensity) (Variables|Default|GetMaxIntensity)))
    (else
      (Rendering|Components|Light|SetIntensity (Variables|Default|GetPointLightComponent) (Math|Interpolation|FInterptoConstant (Variables|/Script/Engine.LightComponentBase|GetIntensity (Variables|Default|GetPointLightComponent)) (Variables|Default|GetTargetIntensity) DeltaSeconds (Variables|Default|GetPulseRate))))))

(fn ConstructionScript)